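; Pond heron hazard actor that moves along a spline and calls RIP on the first-person character when it overlaps them.
; On BeginPlay it finds a HeronPath2_BP in the level and starts a timeline with play rate scaled by TimeToComplete.
; The timeline alpha maps to distance along Spline2, setting the heron's location in world space and its rotation from the spline's local space.
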(event `self.ReceiveActorBeginOverlap`
  (params (OtherActor :type "Actor Object Reference"))
  (bind _asbp_first_person_character (cast `/Game/FirstPerson/Blueprints/BP_FirstPersonCharacter` OtherActor))
  (`/Game/FirstPerson/Blueprints/BP_FirstPersonCharacter.RIP` _asbp_first_person_character))

(event `self.ReceiveBeginPlay`
  (bind _returnvalue (`GameplayStatics.GetActorOfClass` "/Game/Assets/pondStuff/heronPath2_BP.heronPath2_BP_C"))
  (set `self.spline REF2` _returnvalue)
  (`self.Move Heron`))

(event `Move Heron`
  (bind _spline2 (`/Game/Assets/pondStuff/heronPath2_BP.Spline2` (`self.spline REF2`)))
  (`TimelineComponent.SetPlayRate` (`self.Move Heron T`) (/ 1.0 (`self.Time To Complete`)))
  (bind (_direction _move_track) (`Timeline|Move Heron T`)
    (:`Update`
      (bind _returnvalue (`KismetMathLibrary.Lerp` 0.0 (`SplineComponent.GetSplineLength` (`/Game/Assets/pondStuff/heronPath2_BP.Spline2` (`self.spline REF2`))) _move_track))
      (`self.K2_SetActorTransform` (`KismetMathLibrary.MakeTransform` (`SplineComponent.GetLocationAtDistanceAlongSpline` _spline2 _returnvalue "World") (`SplineComponent.GetRotationAtDistanceAlongSpline` _spline2 _returnvalue "Local"))))))

(fn `UserConstructionScript`)