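; Pond heron actor that travels along a spline path and calls RIP on the first-person character when it overlaps them.
; On BeginPlay it finds a HeronPath1_BP in the level and starts MoveHeron.
; A timeline, with play rate set from TimeToComplete, drives distance along that spline to set the heron's transform.
; Location is sampled in world space, but rotation in local space.
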(event `self.ReceiveActorBeginOverlap`
  (params (OtherActor :type "Actor Object Reference"))
  (bind _asbp_first_person_character (cast `/Game/FirstPerson/Blueprints/BP_FirstPersonCharacter` OtherActor))
  (`/Game/FirstPerson/Blueprints/BP_FirstPersonCharacter.RIP` _asbp_first_person_character))

(event `self.ReceiveBeginPlay`
  (bind _returnvalue (`GameplayStatics.GetActorOfClass` "/Game/Assets/pondStuff/heronPath1_BP.heronPath1_BP_C"))
  (set `self.spline REF1` _returnvalue)
  (`self.Move Heron`))

(event `Move Heron`
  (bind _spline1 (`/Game/Assets/pondStuff/heronPath1_BP.Spline1` (`self.spline REF1`)))
  (`TimelineComponent.SetPlayRate` (`self.Move Heron T`) (/ 1.0 (`self.Time To Complete`)))
  (bind (_direction _move_track) (`Timeline|Move Heron T`)
    (:`Update`
      (bind _returnvalue (`KismetMathLibrary.Lerp` 0.0 (`SplineComponent.GetSplineLength` (`/Game/Assets/pondStuff/heronPath1_BP.Spline1` (`self.spline REF1`))) _move_track))
      (`self.K2_SetActorTransform` (`KismetMathLibrary.MakeTransform` (`SplineComponent.GetLocationAtDistanceAlongSpline` _spline1 _returnvalue "World") (`SplineComponent.GetRotationAtDistanceAlongSpline` _spline1 _returnvalue "Local"))))))

(fn `UserConstructionScript`)