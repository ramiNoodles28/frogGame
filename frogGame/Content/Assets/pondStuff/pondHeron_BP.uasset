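; Pond heron hazard actor that travels along a spline path and calls RIP on the first-person character when it overlaps them.
; On BeginPlay it finds a HeronPath_BP in the level and starts moving along that actor's spline.
; A timeline, with play rate scaled by TimeToComplete, lerps distance over the spline length to set the heron's transform, using world-space location but local-space rotation.
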(event `self.ReceiveActorBeginOverlap`
  (params (OtherActor :type "Actor Object Reference"))
  (bind _asbp_first_person_character (cast `/Game/FirstPerson/Blueprints/BP_FirstPersonCharacter` OtherActor))
  (`/Game/FirstPerson/Blueprints/BP_FirstPersonCharacter.RIP` _asbp_first_person_character))

(event `self.ReceiveBeginPlay`
  (bind _returnvalue (`GameplayStatics.GetActorOfClass` "/Game/Assets/pondStuff/heronPath_BP.heronPath_BP_C"))
  (set `self.spline REF` _returnvalue)
  (`self.Move Heron`))

(event `Move Heron`
  (bind _spline (`/Game/Assets/pondStuff/heronPath_BP.Spline` (`self.spline REF`)))
  (`TimelineComponent.SetPlayRate` (`self.Move Heron T`) (/ 1.0 (`self.Time To Complete`)))
  (bind (_direction _move_track) (`Timeline|Move Heron T`)
    (:`Update`
      (bind _returnvalue (`KismetMathLibrary.Lerp` 0.0 (`SplineComponent.GetSplineLength` (`/Game/Assets/pondStuff/heronPath_BP.Spline` (`self.spline REF`))) _move_track))
      (`self.K2_SetActorTransform` (`KismetMathLibrary.MakeTransform` (`SplineComponent.GetLocationAtDistanceAlongSpline` _spline _returnvalue "World") (`SplineComponent.GetRotationAtDistanceAlongSpline` _spline _returnvalue "Local"))))))

(fn `UserConstructionScript`)