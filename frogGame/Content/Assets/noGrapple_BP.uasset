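; Level actor that marks surfaces as non-grappleable and can act as a death plane, such as water.
; On BeginPlay it adds itself to the player BP_FirstPersonCharacter's NoTouch array.
; If its DontTouch mesh is the death plane mesh, it switches collision to OverlapOnlyPawn.
; Any overlap by that character class calls RIP on it to kill the player.
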(event `self.ReceiveBeginPlay`
  ;[0.5469 0 0.01857] Add Self to NoTouch array in the BP_FirstPersonCharacter
  (bind _asbp_first_person_character (cast `/Game/FirstPerson/Blueprints/BP_FirstPersonCharacter` (`GameplayStatics.GetPlayerPawn` 0)))
  (`KismetArrayLibrary.Array_Add` (`/Game/FirstPerson/Blueprints/BP_FirstPersonCharacter.noTouch` _asbp_first_person_character) self)
  ;[1 0 0.3714] If static mesh is a plane (water for example), kill player on collision
  (if (== (`StaticMeshComponent.StaticMesh` (`self.dontTouch`)) (`self.DeathPlaneMesh`))
    (`PrimitiveComponent.SetCollisionProfileName` (`self.dontTouch`) "OverlapOnlyPawn" true)))

(event `self.ReceiveActorBeginOverlap`
  (params (OtherActor :type "Actor Object Reference"))
  ;[1 0 0.3714] If static mesh is a plane (water for example), kill player on collision
  (bind _asbp_first_person_character (cast `/Game/FirstPerson/Blueprints/BP_FirstPersonCharacter` OtherActor))
  (`/Game/FirstPerson/Blueprints/BP_FirstPersonCharacter.RIP` _asbp_first_person_character))

(fn `UserConstructionScript`)